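; Farm door actor that swings open or closed each time its Interact event fires.
; Interact checks IsOpen and plays either the Open or Close timeline from the start.
; Each timeline lerps the Hinge component's relative yaw across a quarter turn and sets IsOpen on every update, so the state flips as the swing begins rather than when it finishes.
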(event EventBeginPlay
  (|CallParentFunction) ; This node is disabled and will not be called.\nDrag off pins to build functionality.
)

(event Collision|EventActorBeginOverlap
  (params (OtherActor :type Actor%20Object%20Reference))
  (|CallParentFunction OtherActor) ; This node is disabled and will not be called.\nDrag off pins to build functionality.
)

(event EventTick
  (params (DeltaSeconds :type Float%20%28single-precision%29))
  (|CallParentFunction DeltaSeconds) ; This node is disabled and will not be called.\nDrag off pins to build functionality.
)

(event EventInteract
  (bind _hinge (Variables|Default|GetHinge))
  (if (Variables|Default|GetisOpen)
    (bind _newtrack_0 (Timeline|Close PlayFromStart)
      (:Update
        (Transformation|SetRelativeRotation _hinge (Math|Rotator|MakeRotator 0.0 0.0 (Math|Float|Lerp -9e+01 0.0 _newtrack_0)) false false)
        (Variables|Default|SetisOpen false)))
    (else
      (bind _newtrack_0_2 (Timeline|Open PlayFromStart)
        (:Update
          (Transformation|SetRelativeRotation _hinge (Math|Rotator|MakeRotator 0.0 0.0 (Math|Float|Lerp 0.0 -9e+01 _newtrack_0_2)) false false)
          (Variables|Default|SetisOpen true))))))

(fn ConstructionScript
  (|CallParentFunction))