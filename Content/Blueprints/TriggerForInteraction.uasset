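; TriggerForInteraction is an interaction point actor with a pop-up prompt widget that relays interaction to a Target.
; BeginPlay caches the widget's scale and hides it by scaling to zero.
; ShowPopup toggles that scale, sets the PopUpText message and uses done flags so the sound plays only on state changes.
; CallTargerInteract calls Interact on a valid Target; an older copy of the pop-up logic sits unconnected in the EventGraph.
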(event EventBeginPlay
  (bind _widget (Variables|Default|GetWidget))
  (Variables|Default|SetCurrentScale (Transformation|GetWorldScale _widget))
  (Transformation|SetWorldScale3D _widget "0, 0, 0"))

(event Collision|EventActorBeginOverlap
  (params (OtherActor :type Actor%20Object%20Reference)))

(event EventTick
  (params (DeltaSeconds :type Float%20%28single-precision%29)))

(fn ConstructionScript)

(fn CallTargerInteract
  (bind _target (Variables|Default|GetTarget))
  (Utilities|IsValid _target
    (:Is%20Valid
      (Default|Interact _target))))

(fn ShowPopup
  (params (ScaleUp :type Boolean))
  (bind _widget (Variables|Default|GetWidget))
  (if ScaleUp
    (if (not (Variables|Default|GetDoneScalingUp))
      (Transformation|SetWorldScale3D _widget (Variables|Default|GetCurrentScale))
      (bind _aspop_up_text (Utilities|Casting|CastToPopUpText (UserInterface|GetUserWidgetObject _widget)))
      (Variables|/Game/UI/PopUpText.PopUpText_C|SetPopUpMessage _aspop_up_text (Variables|Default|GetTextOnPopUP))
      (Variables|Default|SetDoneScalingUp true)
      (Variables|Default|SetDoneScalingDown false)
      (Audio|PlaySoundatLocation "/Game/Audio/PopUp.PopUp" (Transformation|GetWorldLocation (Variables|Default|GetWidget)) "0, 0, 0" 1.0 1.0 0.0 0 0 0 :!label _label))
    (elif (not (Variables|Default|GetDoneScalingDown))
      (Transformation|SetWorldScale3D _widget "0, 0, 0")
      (Variables|Default|SetDoneScalingDown true)
      (Variables|Default|SetDoneScalingUp false)
      (goto _label))))