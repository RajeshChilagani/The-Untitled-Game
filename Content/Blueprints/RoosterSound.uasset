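; RoosterSound is an interactable actor that plays a rooster crow and completes the "Climb Bird House To Sing" task.
; Interact plays the crow, then casts the player character to TUH_BP and checks its Tasks array for that entry.
; If present, it removes the task, plays a check-mark sound and shows a TaskFinish widget for a few seconds before removing it.
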(event EventBeginPlay
  (|CallParentFunction) ; This node is disabled and will not be called.\nDrag off pins to build functionality.
)

(event Collision|EventActorBeginOverlap
  (params (OtherActor :type Actor%20Object%20Reference))
  (|CallParentFunction OtherActor) ; This node is disabled and will not be called.\nDrag off pins to build functionality.
)

(event EventTick
  (params (DeltaSeconds :type Float%20%28single-precision%29))
  (|CallParentFunction DeltaSeconds) ; This node is disabled and will not be called.\nDrag off pins to build functionality.
)

(event EventInteract
  (Audio|PlaySound2D "/Game/Audio/Rooster_sound_Cue.Rooster_sound_Cue" 1.0 1.0 0.0 0 0)
  (bind _astuh_bp (Utilities|Casting|CastToTUH_BP (Game|GetPlayerCharacter 0)))
  (if (!= (Utilities|Array|FindItem (Variables|/Game/TheUntitledHero/TUH_BP.TUH_BP_C|GetTasks _astuh_bp) "Climb Bird House To Sing") -1)
    (Utilities|Array|RemoveItem (Variables|/Game/TheUntitledHero/TUH_BP.TUH_BP_C|GetTasks _astuh_bp) "Climb Bird House To Sing")
    (bind _returnvalue (UserInterface|CreateWidget "/Game/UI/TaskFinish.TaskFinish_C" 0 "Climb Bird House To Sing"))
    (UserInterface|Viewport|AddtoViewport _returnvalue 0)
    (Audio|PlaySound2D "/Game/Audio/Check_mark_sound_effect_Cue.Check_mark_sound_effect_Cue" 1.0 1.0 0.0 0 0)
    (Utilities|FlowControl|Delay 5.0)
    (Widget|RemovefromParent _returnvalue)))

(fn ConstructionScript
  (|CallParentFunction))