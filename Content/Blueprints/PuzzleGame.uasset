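; Timed puzzle trigger actor: when the UH_BP character overlaps its box, it slows time, shows the puzzle UI and prompts to press Enter.
; Tick uses a Delay as a one-second countdown while PuzzleStarted is set; timeout plays a sound and resets with a retry prompt.
; PuzzleStarted and FinishedPuzzle are only cleared here, never set true; finishing hides the UI.
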(event OnComponentBeginOverlap(Box)
  (params (OverlappedComponent :type Primitive%20Component%20Object%20Reference) (OtherActor :type Actor%20Object%20Reference) (OtherComp :type Primitive%20Component%20Object%20Reference) (OtherBodyIndex :type Integer) (bFromSweep :type Boolean) (SweepResult :type Hit%20Result%20Structure%20%28by%20ref%29))
  (if (not (Variables|Default|GetStartPuzzle))
    (Utilities|Casting|CastToTUH_BP OtherActor)
    (Variables|Default|SetStartPuzzle true)
    (Variables|Default|SetRestartPuzzle false)
    (CallFunction|StartPuzzleFunc "Finish the Puzzle In Time 
Press Enter to Start")
    (CallFunction|ShowUI)
    (Audio|PlaySound2D "/Game/Audio/TaskUI.TaskUI" 1.0 1.0 0.0 0 0)))

(event EventBeginPlay
  (Variables|Default|SetTimeToFinish (Variables|Default|GetTime)))

(event Collision|EventActorBeginOverlap
  (params (OtherActor :type Actor%20Object%20Reference)))

(event EventTick
  (params (DeltaSeconds :type Float%20%28single-precision%29))
  (bind _timetofinish (Variables|Default|GetTimeToFinish))
  (if (Variables|Default|GetPuzzleStarted)
    (if (Variables|Default|GetFinishedPuzzle)
      (Widget|SetVisibility (Variables|Default|GetPuzzleUI) "Hidden")
      (Variables|Default|SetStartPuzzle false)
      (else
        (Utilities|FlowControl|Delay 1.0)
        (if (>= _timetofinish 1)
          (Math|Integer|DecrementInt _timetofinish)
          (else
            (CallFunction|Restart)))))))

(fn ConstructionScript)

(fn StartPuzzleFunc
  (params (MainText :type Text))
  (Variables|Default|SetInfoText MainText)
  (Variables|Default|SetPuzzleStarted false)
  (Variables|Default|SetFinishedPuzzle false)
  (Variables|Default|SetTimeToFinish (Variables|Default|GetTime))
  (Utilities|Time|SetGlobalTimeDilation 0.1))

(fn ShowUI
  (Utilities|IsValid (Variables|Default|GetPuzzleUI)
    (:Is%20Valid
      (if (Widget|IsVisible (Variables|Default|GetPuzzleUI))
        _
        (else
          (Widget|SetVisibility (Variables|Default|GetPuzzleUI) "Visible"))))
    (:Is%20Not%20Valid
      (bind _returnvalue (UserInterface|CreateWidget "/Game/UI/PuzzleUI.PuzzleUI_C"))
      (Variables|Default|SetPuzzleUI _returnvalue)
      (UserInterface|Viewport|AddtoViewport _returnvalue 0)))
  (Class|Image|SetOpacity (Variables|/Game/UI/PuzzleUI.PuzzleUI_C|GetImage_32 (Variables|Default|GetPuzzleUI)) 1.0))

(fn HideUI)

(fn Restart
  (Audio|PlaySound2D "/Game/Audio/busted_Cue.busted_Cue" 2.0 1.0 0.0 0 0)
  (CallFunction|StartPuzzleFunc "OOPS! TimeUp 
Press Enter to Try Again")
  (CallFunction|ShowUI)
  (Variables|Default|SetStartPuzzle false)
  (Variables|Default|SetRestartPuzzle true))