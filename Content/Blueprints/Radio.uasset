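; Interactable radio actor that plays music through a media player and can complete a player task.
; On BeginPlay it lowers the media sound volume; the first Interact opens the radio playlist and later ones skip to the next track.
; Turning it on also removes the "Play Music From Radio" task from the TUH_BP player character, showing a timed TaskFinish widget with a checkmark sound.
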(event EventBeginPlay
  (Audio|Components|Audio|SetVolumeMultiplier (Variables|Default|GetMediaSound) 0.1 :!class /Script/AudioMixer.SynthComponent))

(event Collision|EventActorBeginOverlap
  (params (OtherActor :type Actor%20Object%20Reference)))

(event EventTick
  (params (DeltaSeconds :type Float%20%28single-precision%29)))

(event EventInteract
  (bind _radiomp (Variables|Default|GetRadioMP))
  (if (Variables|Default|GetIsON)
    (Class|MediaPlayer|Next _radiomp)
    (else
      (Class|MediaPlayer|OpenPlaylistIndex _radiomp "/Game/Audio/RadioPlaylist/RadioPlaylist.RadioPlaylist")
      (Variables|Default|SetIsON true)
      (bind _astuh_bp (Utilities|Casting|CastToTUH_BP (Game|GetPlayerCharacter 0)))
      (if (!= (Utilities|Array|FindItem (Variables|/Game/TheUntitledHero/TUH_BP.TUH_BP_C|GetTasks _astuh_bp) "Play Music From Radio") -1)
        (Utilities|Array|RemoveItem (Variables|/Game/TheUntitledHero/TUH_BP.TUH_BP_C|GetTasks _astuh_bp) "Play Music From Radio")
        (bind _returnvalue (UserInterface|CreateWidget "/Game/UI/TaskFinish.TaskFinish_C" 0 "Play Music From Radio"))
        (UserInterface|Viewport|AddtoViewport _returnvalue 0)
        (Audio|PlaySound2D "/Game/Audio/Check_mark_sound_effect_Cue.Check_mark_sound_effect_Cue" 1.0 1.0 0.0 0 0)
        (Utilities|FlowControl|Delay 5.0)
        (Widget|RemovefromParent _returnvalue)))))

(fn ConstructionScript)