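; Task trigger volume that completes a named task when a TUH_BP actor overlaps it, with box size set from X, Y and Z in the construction script.
; Each overlap removes Task from that actor's Tasks list, without checking that it was present.
; A DoOnce limits the feedback to the first such overlap: a TaskFinish widget naming the task and a check-mark sound, with the widget removed after a short delay.
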(event OnComponentBeginOverlap(Trigger)
  (params (OverlappedComponent :type Primitive%20Component%20Object%20Reference) (OtherActor :type Actor%20Object%20Reference) (OtherComp :type Primitive%20Component%20Object%20Reference) (OtherBodyIndex :type Integer) (bFromSweep :type Boolean) (SweepResult :type Hit%20Result%20Structure%20%28by%20ref%29))
  (bind _task (Variables|Default|GetTask))
  (bind _astuh_bp (Utilities|Casting|CastToTUH_BP OtherActor))
  (Utilities|Array|RemoveItem (Variables|/Game/TheUntitledHero/TUH_BP.TUH_BP_C|GetTasks _astuh_bp) _task)
  (Utilities|FlowControl|DoOnce false
    (:Completed
      (bind _returnvalue (UserInterface|CreateWidget "/Game/UI/TaskFinish.TaskFinish_C" 0 (Utilities|Text|ToText(String) _task)))
      (UserInterface|Viewport|AddtoViewport _returnvalue 0)
      (Audio|PlaySound2D "/Game/Audio/Check_mark_sound_effect_Cue.Check_mark_sound_effect_Cue" 1.0 1.0 0.0 0 0)
      (Utilities|FlowControl|Delay 5.0)
      (Widget|RemovefromParent _returnvalue))))

(event EventBeginPlay)

(event Collision|EventActorBeginOverlap
  (params (OtherActor :type Actor%20Object%20Reference)))

(fn ConstructionScript
  (Components|Box|SetBoxExtent (Variables|Default|GetTrigger) (Math|Vector|MakeVector (Variables|Default|GetX) (Variables|Default|GetY) (Variables|Default|GetZ)) true))